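; BP_Guard1 is a guard Blueprint with three states: patrol to the top and back, wait for the other guard to die, and move toward the treasure.
; Custom events set CurrentState to wait or treasure, with the treasure switch first teleporting the guard to SwooshToPosition and skipping if already in that state.
; A separate event unpossesses its AI controller; the movement for each state is not implemented in this graph.
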(event Custom|Unpossess%20event
  ;[1 1 1] Unpossess the AI controller
  (Pawn|UnPossess (AI|GetAIController self)))

(event Custom|ChangeStateToWait
  ;[1 1 1] 3 states for Guard1. First move to the top and back (currentState = 0).
  ; Second is to wait till the other guard dies  (currentState = 1).
  ; Third is to move towards the treasure (currentState = 2)
  (Variables|Default|SetcurrentState 1))

(event Custom|ChangeStateToMoveToTreasure
  ;[1 1 1] 3 states for Guard1. First move to the top and back (currentState = 0).
  ; Second is to wait till the other guard dies  (currentState = 1).
  ; Third is to move towards the treasure (currentState = 2)
  (if (not (== (Variables|Default|GetcurrentState) 2))
    (Transformation|Teleport (Variables|Default|GetSwooshToPosition) "0, 0, 0")
    (Variables|Default|SetcurrentState 2)))

(event EventBeginPlay)

(event Collision|EventActorBeginOverlap
  (params (OtherActor :type Actor%20Object%20Reference)))

(event EventTick
  (params (DeltaSeconds :type Float%20%28single-precision%29)))

(fn ConstructionScript)